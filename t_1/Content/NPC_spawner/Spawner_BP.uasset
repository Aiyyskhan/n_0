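; Spawner actor that creates an NPC of a configurable class at its own location and rotation.
; Every Tick calls SpawnNPC, which spawns only while the Make flag is set, then clears it so each trigger yields one NPC.
; The spawn adjusts for collisions but always succeeds, and the new NPC receives the spawner's TargetObject.
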(event EventTick
  (params (DeltaSeconds :type Float%20%28single-precision%29))
  (CallFunction|SpawnNPC))

(fn ConstructionScript)

(fn SpawnNPC
  (if (Variables|Default|Getmake)
    (bind _returnvalue (Game|SpawnActorfromClass (Variables|Default|GetNPC_to_spawn) (Math|Transform|MakeTransform (Transformation|GetActorLocation) (Transformation|GetActorRotation)) "AdjustIfPossibleButAlwaysSpawn" 0 0))
    (Variables|/Game/NPC/NPC_BaseBP.NPC_BaseBP_C|Settarget_object _returnvalue (Variables|Default|Gettarget_object))
    (Variables|Default|Setmake false)))